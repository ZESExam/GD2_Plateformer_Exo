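; BP_Key is a key pickup actor that sets HadKey on BP_GameInstance and destroys itself when interacted with.
; On BeginPlay it caches the game instance and game mode, creates an interact widget and adds a BPW_Clé key widget to the viewport.
; Interact also passes the key widget to the game mode through GetWidgetRef.
; ShowText displays the interact widget with a "Press E" prompt.
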(event `self.ReceiveBeginPlay`
  (bind _returnvalue (`|CreateWidget` "/Game/GAME/Bluprints/Widget/BPW_Interact.BPW_Interact_C"))
  (set `self.Ref_BPW_Interact` _returnvalue)
  (bind _asbp_game_instance (cast `/Game/GAME/Bluprints/BP_GameInstance` (`GameplayStatics.GetGameInstance`)))
  (set `self.As BP Game Instance` _asbp_game_instance)
  (bind _returnvalue_2 (`|CreateWidget` "/Game/GAME/Bluprints/Widget/BPW_Clé.BPW_Clé_C"))
  (`UserWidget.AddToViewport` _returnvalue_2 0)
  (set `self.WidgetRef` _returnvalue_2)
  (bind _asbp_game_mode (cast `/Game/GAME/Bluprints/BP_GameMode` (`GameplayStatics.GetGameMode`)))
  (set `self.As BP Game Mode` _asbp_game_mode))

(event `/Game/GAME/Bluprints/BPI/BPI_Interact.Interact`
  (set `/Game/GAME/Bluprints/BP_GameInstance.HadKey?` true (`self.As BP Game Instance`))
  (`self.K2_DestroyActor`)
  (`/Game/GAME/Bluprints/BP_GameMode.GetWidgetRef` (`self.As BP Game Mode`) (`self.WidgetRef`)))

(fn `Show_Text`
  (bind _ref_bpw_interact (`self.Ref_BPW_Interact`))
  (set `TextBlock.Text` "Press E" (`/Game/GAME/Bluprints/Widget/BPW_Interact.Txt_Interact` _ref_bpw_interact))
  (`UserWidget.AddToViewport` _ref_bpw_interact 0))

(fn `UserConstructionScript`)