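; BP_door is a door actor whose position follows a shared door state held in BP_GameInstance.
; On BeginPlay it binds to the game instance's OnLightToogle event and syncs immediately, so each light toggle re-reads GetDoorState.
; UpdateDoorState then snaps the Cube between a raised and a lowered relative location, with no interpolation or sweep.
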(event `self.ReceiveBeginPlay`
  (bind _asbp_game_instance (cast `/Game/GAME/Bluprints/BP_GameInstance` (`GameplayStatics.GetGameInstance`)))
  (bind _output_get (set `self.As BP Game Instance` _asbp_game_instance))
  (add `/Game/GAME/Bluprints/BP_GameInstance.OnLightToogle` _output_get (delegate `ToggleDoorState`))
  (`self.UpdateDoorState`))

(event `ToggleDoorState`
  (`self.UpdateDoorState`))

(fn `UpdateDoorState`
  (bind _doorstate (`/Game/GAME/Bluprints/BP_GameInstance.GetDoorState` (`self.As BP Game Instance`)))
  (if _doorstate
    (`SceneComponent.K2_SetRelativeLocation` (`self.Cube`) (0.0 0.0 280.0) false false)
    (else
      (`SceneComponent.K2_SetRelativeLocation` (`self.Cube`) (0.0 0.0 100.0) false false))))

(fn `UserConstructionScript`)