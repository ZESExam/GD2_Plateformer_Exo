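; BP_lightEnigme is a light actor, apparently for a puzzle, whose PointLight visibility follows a numbered light state held in BP_GameInstance.
; On BeginPlay it caches the game instance, binds to its OnLightToogle event and applies the initial state.
; Each toggle event makes it query the state for its LightNumber and update visibility, so it needs no Tick.
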(event `self.ReceiveBeginPlay`
  (bind _asbp_game_instance (cast `/Game/GAME/Bluprints/BP_GameInstance` (`GameplayStatics.GetGameInstance`)))
  (bind _output_get (set `self.As BP Game Instance` _asbp_game_instance))
  (add `/Game/GAME/Bluprints/BP_GameInstance.OnLightToogle` _output_get (delegate `ToogleLightState`))
  (`self.UpdateLightState`))

(event `ToogleLightState`
  (`self.UpdateLightState`))

(fn `UpdateLightState`
  (bind _lightstate (`/Game/GAME/Bluprints/BP_GameInstance.GetLightStateByNumber` (`self.As BP Game Instance`) (`self.LightNumber`)))
  (`SceneComponent.SetVisibility` (`self.PointLight`) _lightstate false))

(fn `UserConstructionScript`)